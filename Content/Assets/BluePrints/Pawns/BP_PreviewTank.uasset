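; BP_PreviewTank is a preview tank pawn whose turret idly sweeps around its starting heading and which fires on the PreviewFire input.
; A looping timer started at BeginPlay periodically picks a random yaw within a fixed arc around the initial turret yaw.
; Tick eases the turret mesh toward that target with RInterpTo, keeping the target's pitch and roll from the turret's current rotation.
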(event EventBeginPlay
  (Variables|Default|SetInitialTurretZRotation (.Yaw (Math|Rotator|BreakRotator (Transformation|GetWorldRotation (Variables|Default|GetTurretMesh)))))
  (CallFunction|SetTargetTurretRotation)
  (Utilities|Time|SetTimerbyFunctionName 0 "SetTargetTurretRotation" 3.0 true))

(event EventTick
  (params (DeltaSeconds :type Float%20%28single-precision%29))
  (Transformation|SetWorldRotation (Variables|Default|GetTurretMesh) (Math|Interpolation|RInterpTo (Transformation|GetWorldRotation (Variables|Default|GetTurretMesh)) (Variables|Default|GetTargetTurretRotation) DeltaSeconds 1.0) false false))

(event Input|ActionEvents|InputActionPreviewFire
  (params (Key :type Key%20Structure))
  (:Pressed
    (Class|BasePawn|Fire)))

(fn ConstructionScript)

(fn SetTargetTurretRotation
  (bind _turretmesh (Variables|Default|GetTurretMesh))
  (bind _returnvalue (Transformation|GetWorldRotation _turretmesh))
  (bind (_roll _pitch) (Math|Rotator|BreakRotator _returnvalue))
  (Variables|Default|SetTargetTurretRotation (Math|Rotator|MakeRotator _roll _pitch (+ (Variables|Default|GetInitialTurretZRotation) (Math|Random|RandomFloatinRange -6e+01 6e+01)))))